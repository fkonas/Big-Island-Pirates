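; Main menu pawn that shows the W_MainMenu widget with mouse cursor and game-and-UI input on BeginPlay.
; It caches two camera transforms, then SetActiveCam and SetMainMenuCam play a timeline forward or backward to move the main camera between them.
; The timeline track feeds VInterpTo and RInterpTo as DeltaTime, acting as a blend alpha.
; SetQualitySetting forwards quality changes to the menu's options widget.
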(event EventBeginPlay
  (bind _returnvalue (Game|GetPlayerController 0))
  (bind _camera (Variables|Default|GetCamera))
  (bind _camera1 (Variables|Default|GetCamera1))
  (Utilities|FlowControl|Sequence
    (:then_0
      (bind _returnvalue_2 (UserInterface|CreateWidget "/Game/_Core/Widget/MainMenu/W_MainMenu.W_MainMenu_C" (Game|GetPlayerController 0)))
      (bind _output_get (Variables|Default|SetMainMenuRef _returnvalue_2))
      (UserInterface|Viewport|AddtoViewport _output_get 0)
      (Input|SetInputModeGameandUI _returnvalue 0 "DoNotLock" true false)
      (Variables|/Script/Engine.PlayerController|SetbShowMouseCursor _returnvalue true))
    (:then_1
      (Variables|Default|SetStartCamLocation (Transformation|GetWorldLocation _camera))
      (Variables|Default|SetEndCamLocation (Transformation|GetWorldLocation _camera1))
      (Variables|Default|SetStartRotation (Variables|/Script/Engine.SceneComponent|GetRelativeRotation _camera))
      (Variables|Default|SetEndRotation (Variables|/Script/Engine.SceneComponent|GetRelativeRotation _camera1)))))

(event EventSetMainMenuCam
  (bind _camera (Variables|Default|GetCamera))
  (bind _newtrack_0 (Timeline|Timeline ReverseFromEnd)
    (:Update
      (Transformation|SetWorldLocation _camera (Math|Interpolation|VInterpTo (Variables|Default|GetStartCamLocation) (Variables|Default|GetEndCamLocation) _newtrack_0 1.0) false false)
      (Transformation|SetRelativeRotation _camera (Math|Interpolation|RInterpTo (Variables|Default|GetStartRotation) (Variables|Default|GetEndRotation) _newtrack_0 1.0) false false))))

(event EventSetActiveCam
  (bind _camera (Variables|Default|GetCamera))
  (bind _newtrack_0 (Timeline|Timeline PlayFromStart)
    (:Update
      (Transformation|SetWorldLocation _camera (Math|Interpolation|VInterpTo (Variables|Default|GetStartCamLocation) (Variables|Default|GetEndCamLocation) _newtrack_0 1.0) false false)
      (Transformation|SetRelativeRotation _camera (Math|Interpolation|RInterpTo (Variables|Default|GetStartRotation) (Variables|Default|GetEndRotation) _newtrack_0 1.0) false false))))

(event EventSetQualitySetting
  (params (Setting :type E_GraphicSettings%20Enum :default "NewEnumerator0") (Quality :type Integer))
  (Default|SetQuality (Variables|/Game/_Core/Widget/MainMenu/W_MainMenu.W_MainMenu_C|GetOptionsWidget (Variables|Default|GetMainMenuRef)) Setting Quality))

(fn ConstructionScript)