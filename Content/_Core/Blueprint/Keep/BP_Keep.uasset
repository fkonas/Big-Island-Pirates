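; BP_Keep is the keep the player must protect, losing Health to skeleton attacks and triggering game over when it falls.
; Its AnyDamage event only counts damage from causers tagged Skeleton, then pushes scaled Health to the health bar on its widget component.
; When Health reaches zero or below, it also sends GameOverMessage to the game mode.
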(event Game|Damage|EventAnyDamage
  (params (Damage :type Float%20%28single-precision%29) (DamageType :type Damage%20Type%20Object%20Reference) (InstigatedBy :type Controller%20Object%20Reference) (DamageCauser :type Actor%20Object%20Reference))
  ;[0 0 0] Keep Receive Damage, Update Health Bar
  (if (Actor|ActorHasTag DamageCauser "Skeleton")
    (if (<= (- (Variables|Default|GetHealth) Damage) 0.0)
      (Variables|Default|SetHealth (- (Variables|Default|GetHealth) Damage))
      (Class|BPIHealthBarInterface|UpdateHealth(Message) (UserInterface|GetUserWidgetObject (Variables|Default|GetWidget)) (* (Variables|Default|GetHealth) 0.1))
      (Class|BPITowerDefenceGameMode|GameOver(Message) (Game|GetGameMode) true)
      (else
        (Variables|Default|SetHealth (- (Variables|Default|GetHealth) Damage))
        (Class|BPIHealthBarInterface|UpdateHealth(Message) (UserInterface|GetUserWidgetObject (Variables|Default|GetWidget)) (* (Variables|Default|GetHealth) 0.1))))))

(fn ConstructionScript)