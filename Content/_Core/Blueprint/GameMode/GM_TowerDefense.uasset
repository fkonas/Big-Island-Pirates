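; Tower defense game mode that runs the skeleton wave loop and reports progress and results to the player character's UI.
; Each wave spawns four skeletons per wave number at random BP_SpawnPoint actors, starting at BeginPlay before the character reference is cached.
; SkeletonKilled counts deaths; a cleared wave either wins on the final wave or starts a timed pre-round break.
; When the timer ends, the next wave spawns and buy mode stops.
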(event Custom|SpawnSkeleton
  (bind _characterref (Variables|Default|GetCharacterRef))
  ;[0 0 0] Spawn Skeletons in Game
  (bind _output_get (Variables|Default|SetSkeletonTotal (* (Variables|Default|GetCurrentWave) 4)))
  (Variables|Default|SetSkeletonLeft _output_get)
  (for _index (range 1 (Variables|Default|GetSkeletonTotal))
    (Game|SpawnActorfromClass "/Game/_Core/Blueprint/Skeleton/BP_Skeleton.BP_Skeleton_C" (Math|Transform|MakeTransform (Transformation|GetActorLocation (.OutItem (Utilities|Array|Random (Variables|Default|GetSpawnPoints)))) "0, 0, 0" "1.000000,1.000000,1.000000") "Undefined" "MultiplyWithRoot" 0 0))
  (Utilities|IsValid _characterref
    (:Is%20Valid
      (Class|BPIPirateCharacter|UpdateSkeletonsUI(Message) _characterref (Variables|Default|GetSkeletonLeft) (Variables|Default|GetSkeletonTotal)))))

(event Custom|WaveIncrement
  (bind _characterref (Variables|Default|GetCharacterRef))
  ;[0 0 0] Check if Player Won Game, Start Next Wave
  (if (== (Variables|Default|GetCurrentWave) (Variables|Default|GetMaxWave))
    (CallFunction|GameOver false)
    (else
      (Math|Integer|IncrementInt (Variables|Default|GetCurrentWave)
        (:%20%20
          (CallFunction|PreRoundTimer)))))
  (Utilities|IsValid _characterref
    (:Is%20Valid
      (Class|BPIPirateCharacter|UpdateWavesUI(Message) _characterref (Variables|Default|GetCurrentWave) (Variables|Default|GetMaxWave)))))

(event Custom|PreRoundTimer
  (bind _characterref (Variables|Default|GetCharacterRef))
  ;[0 0 0] Coutdown to Starting Next Wave
  (Utilities|IsValid _characterref
    (:Is%20Valid
      (Class|BPIPirateCharacter|NextRoundStarting(Message) _characterref))
    (:Is%20Not%20Valid
      _))
  (Utilities|Time|SetTimerbyEvent (delegate Custom|StartNextWave) 3e+01))

(event Custom|StartNextWave
  (bind _characterref (Variables|Default|GetCharacterRef))
  ;[0 0 0] Coutdown to Starting Next Wave
  (CallFunction|SpawnSkeleton)
  (Utilities|IsValid _characterref
    (:Is%20Valid
      (Default|StopBuyMode _characterref))))

(event EventBeginPlay
  ;[0 0 0] Event Begin Play, Set References
  (Utilities|FlowControl|Sequence
    (:then_0
      (bind _outactors (Actor|GetAllActorsOfClass "/Game/_Core/Blueprint/Skeleton/BP_SpawnPoint.BP_SpawnPoint_C"))
      (Variables|Default|SetSpawnPoints _outactors)
      (CallFunction|SpawnSkeleton))
    (:then_1
      (bind _outactors_2 (Actor|GetAllActorsOfClass "/Game/_Core/Blueprint/BP_ThirdPersonCharacter.BP_ThirdPersonCharacter_C"))
      (Variables|Default|SetCharacterRef (Utilities|Array|Get(acopy) _outactors_2)))))

(event EventGameOver
  (params (LostGame? :type Boolean))
  (bind _characterref (Variables|Default|GetCharacterRef))
  ;[0 0 0] Show Win Or Lose Scrren On Player Widget
  (Utilities|IsValid _characterref
    (:Is%20Valid
      (Class|BPIPirateCharacter|WinorLoseGame(Message) _characterref (not LostGame?)))))

(event EventSkeletonKilled
  (bind _characterref (Variables|Default|GetCharacterRef))
  ;[0 0 0] Count Skeletons Killed
  (bind _result (Math|Integer|DecrementInt (Variables|Default|GetSkeletonLeft))
    (:%20%20
      (if (== _result 0)
        (Development|PrintString "All Skeletons are killed, New wave is starting soon" true true "(R=1.000000,G=0.485572,B=0.000000,A=1.000000)" 5.0)
        (CallFunction|WaveIncrement))
      (Utilities|IsValid _characterref
        (:Is%20Valid
          (Class|BPIPirateCharacter|UpdateSkeletonsUI(Message) _characterref (Variables|Default|GetSkeletonLeft) (Variables|Default|GetSkeletonTotal)))))))

(fn ConstructionScript)