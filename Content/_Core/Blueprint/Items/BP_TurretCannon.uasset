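; BP_TurretCannon is an automated turret that locks onto the first Skeleton-tagged pawn its PawnSensing sees while it has no target.
; A fast looping timer turns its yaw toward the target, releasing the lock once that pawn is invalid.
; A slower timer spawns BP_CannonBall at the Arrow with a sound, stopping when the target is invalid or reports dead through a message call.
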(event OnSeePawn(PawnSensing)
  (params (Pawn :type Pawn%20Object%20Reference))
  ;[0 0 0] Event See Target
  (if (Actor|ActorHasTag Pawn "Skeleton")
    (Utilities|IsValid Pawn
      (:Is%20Valid
        (if (not (Variables|Default|GetHasTarget?))
          (Variables|Default|SetHasTarget? true)
          (Variables|Default|SetTargetPawn Pawn)
          (CallFunction|TrackTarget)
          (CallFunction|FireLoop))))))

(event Custom|TrackTarget
  ;[0 0 0] Rotate Cannon to Face Target
  (bind _returnvalue (Utilities|Time|SetTimerbyEvent (delegate Custom|MoveTurret) 0.05 true true))
  (Variables|Default|SetTimerRef _returnvalue))

(event Custom|MoveTurret
  (bind _targetpawn (Variables|Default|GetTargetPawn))
  ;[0 0 0] Rotate Cannon to Face Target
  (Utilities|IsValid _targetpawn
    (:Is%20Valid
      (Transformation|SetActorRotation (Math|Rotator|MakeRotator 0.0 0.0 (.yaw (Math|Interpolation|RInterpTo (Transformation|GetActorRotation) (Math|Rotator|FindLookatRotation (Transformation|GetActorLocation) (Transformation|GetActorLocation _targetpawn)) (Utilities|Time|GetWorldDeltaSeconds) 1e+02)))))
    (:Is%20Not%20Valid
      (Utilities|Time|ClearandInvalidateTimerbyHandle (Variables|Default|GetTimerRef))
      (Variables|Default|SetHasTarget? false))))

(event Custom|FireLoop
  ;[0 0 0] Fire Loop Logic
  (bind _returnvalue (Utilities|Time|SetTimerbyEvent (delegate Custom|FireCannon) 4.0 true))
  (Variables|Default|SetFireTimeRef _returnvalue))

(event Custom|FireCannon
  ;[0 0 0] Fire Loop Logic
  (if (Variables|Default|GetHasTarget?)
    (bind _targetpawn (Variables|Default|GetTargetPawn)
      (:then
        (bind _isdead_ (Class|BPISkeletonCharacter|GetIsSkeletonDead?(Message) _targetpawn))
        (if _isdead_
          (Utilities|Time|ClearandInvalidateTimerbyHandle (Variables|Default|GetFireTimeRef))
          (else
            (Game|SpawnActorfromClass "/Game/_Core/Blueprint/Items/BP_CannonBall.BP_CannonBall_C" (Transformation|GetWorldTransform (Variables|Default|GetArrow)) "Undefined" "MultiplyWithRoot" 0 0)
            (Audio|PlaySound2D "/Game/MilitaryWeapDark/Sound/RocketLauncher/RocketLauncherB_Fire_Cue.RocketLauncherB_Fire_Cue" 1.0 1.0 0.0 0 0))))
      (:else
        (Utilities|Time|ClearandInvalidateTimerbyHandle (Variables|Default|GetFireTimeRef) :!label _label)))
    (else
      (goto _label))))

(fn ConstructionScript)